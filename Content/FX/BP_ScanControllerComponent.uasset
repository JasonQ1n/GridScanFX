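; Player controller component that drives a fade-in/fade-out scan effect around the controlled pawn.
; StartScan and EndScan switch a state machine, whose Tick advances normalized time and is disabled when faded out.
; Time, state flags and pawn location feed the MPC_Scan parameter collection.
; A lazily spawned BP_ScanActor carries the dynamic post-process material, blended by an optional curve, and grid-snapped Niagara, and is optionally destroyed after fade-out.
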(event EventBeginPlay
  (bind _asplayer_controller (Utilities|Casting|CastToPlayerController (Components|GetOwner))
    (:then
      (Variables|Default|SetAs%20Player%20Controller _asplayer_controller)
      (CallFunction|UpdateScanState "NewEnumerator3" true)
      (Rendering|Material|SetScalarParameterValue "/Game/FX/MPC_Scan.MPC_Scan" "GridCellSize" (Variables|Default|GetGridCellSize) :!class /Script/Engine.KismetMaterialLibrary)
      (Rendering|Material|SetScalarParameterValue "/Game/FX/MPC_Scan.MPC_Scan" "Range" (Variables|Default|GetRange) :!class /Script/Engine.KismetMaterialLibrary))
    (:CastFailed
      (CallFunction|UpdateScanState "NewEnumerator4" true))))

(event EventTick
  (params (DeltaSeconds :type Float%20%28single-precision%29))
  (CallFunction|UpdateScanTime DeltaSeconds)
  (Development|PrintString (Utilities|String|Append (Utilities|String|EnumtoString (Variables|Default|GetState)) (Utilities|String|ToString(Float) (Variables|Default|GetScanNormalizedTime))) true false "(R=0.000000,G=0.660000,B=1.000000,A=1.000000)" 0.0)
  (switch Utilities|FlowControl|Switch|SwitchonEBP_ScanState (CallFunction|GetScanState)
    (:NewEnumerator0
      (CallFunction|UpdateScanPPBlendWeight :!label _label))
    (:NewEnumerator1
      _)
    (:NewEnumerator2
      (goto _label))
    (:NewEnumerator3
      _))
  (CallFunction|UpdateScanLocation))

(fn StartScan
  (switch Utilities|FlowControl|Switch|SwitchonEBP_ScanState (CallFunction|GetScanState)
    (:NewEnumerator2
      _)
    (:NewEnumerator3
      _))
  (CallFunction|UpdateScanState "NewEnumerator0" false))

(fn EndScan
  (switch Utilities|FlowControl|Switch|SwitchonEBP_ScanState (CallFunction|GetScanState)
    (:NewEnumerator0
      _)
    (:NewEnumerator1
      _))
  (CallFunction|UpdateScanState "NewEnumerator2" false))

(fn GetScanState
  (return (Variables|Default|GetState)))

(fn UpdateScanState
  (params (State :type EBP_ScanState%20Enum :default "NewEnumerator0") (Force :type Boolean))
  (if (or (Utilities|Enum|NotEqual(Enum) State (Variables|Default|GetState)) Force)
    (Utilities|FlowControl|Sequence
      (:then_0
        (switch Utilities|FlowControl|Switch|SwitchonEBP_ScanState (Variables|Default|GetState)
          (:NewEnumerator1
            (Rendering|Material|SetScalarParameterValue "/Game/FX/MPC_Scan.MPC_Scan" "bFadedIn" 0.0 :!class /Script/Engine.KismetMaterialLibrary))
          (:NewEnumerator3
            (Rendering|Material|SetScalarParameterValue "/Game/FX/MPC_Scan.MPC_Scan" "bFadedOut" 0.0 :!class /Script/Engine.KismetMaterialLibrary)
            (Components|Tick|SetComponentTickEnabled true))))
      (:then_1
        (bind _output_get (Variables|Default|SetState State))
        (switch Utilities|FlowControl|Switch|SwitchonEBP_ScanState _output_get
          (:NewEnumerator1
            (Rendering|Material|SetScalarParameterValue "/Game/FX/MPC_Scan.MPC_Scan" "bFadedIn" 1.0 :!class /Script/Engine.KismetMaterialLibrary)
            (CallFunction|UpdateScanPPBlendWeight))
          (:NewEnumerator3
            (Rendering|Material|SetScalarParameterValue "/Game/FX/MPC_Scan.MPC_Scan" "bFadedOut" 1.0 :!class /Script/Engine.KismetMaterialLibrary)
            (CallFunction|UpdateScanPPBlendWeight)
            (Components|Tick|SetComponentTickEnabled false :!label _label)
            (CallFunction|DestroyPPActor))
          (:NewEnumerator4
            (goto _label))))
      (:then_2
        (return true)))
    (else
      (return false))))

(fn UpdateScanTime
  (params (DeltaTime :type Float%20%28double-precision%29))
  (Utilities|FlowControl|Sequence
    (:then_0
      (switch Utilities|FlowControl|Switch|SwitchonEBP_ScanState (CallFunction|GetScanState)
        (:NewEnumerator0
          (bind _output_get (Variables|Default|SetScanNormalizedTime (+ (Variables|Default|GetScanNormalizedTime) (* DeltaTime (Variables|Default|GetFadeInSpeed)))))
          (if (> _output_get 1.0)
            (Variables|Default|SetScanNormalizedTime 1.0)
            (CallFunction|UpdateScanState "NewEnumerator1" false)))
        (:NewEnumerator2
          (bind _output_get_2 (Variables|Default|SetScanNormalizedTime (- (Variables|Default|GetScanNormalizedTime) (* DeltaTime (Variables|Default|GetFadeOutSpeed)))))
          (if (< _output_get_2 0.0)
            (Variables|Default|SetScanNormalizedTime 0.0)
            (CallFunction|UpdateScanState "NewEnumerator3" false)))
        (:NewEnumerator4
          (return false)))
      (Rendering|Material|SetScalarParameterValue "/Game/FX/MPC_Scan.MPC_Scan" "NormalizedTime" (Variables|Default|GetScanNormalizedTime) :!class /Script/Engine.KismetMaterialLibrary))
    (:then_1
      (return true))))

(fn GetScanPPActor
  (bind _ppmaterial (Variables|Default|GetPPMaterial))
  (Utilities|IsValid (Variables|Default|GetScan%20Actor)
    (:Is%20Valid
      (return (Variables|Default|GetScan%20Actor)))
    (:Is%20Not%20Valid
      (bind _returnvalue (Game|SpawnActorfromClass "/Game/FX/BP_ScanActor.BP_ScanActor_C" (Math|Transform|MakeTransform "0, 0, 0") "Undefined" "MultiplyWithRoot" 0 0))
      (Variables|Default|SetScan%20Actor _returnvalue)
      (Utilities|FlowControl|Sequence
        (:then_0
          (Utilities|IsValid (Variables|Default|GetPPMID)
            (:Is%20Valid
              _)
            (:Is%20Not%20Valid
              (Utilities|IsValid _ppmaterial
                (:Is%20Valid
                  (bind _returnvalue_2 (Rendering|Material|CreateDynamicMaterialInstance _ppmaterial "None" "None" :!class /Script/Engine.KismetMaterialLibrary))
                  (Variables|Default|SetPPMID _returnvalue_2)))))
          (Utilities|IsValid (Variables|/Game/FX/BP_ScanActor.BP_ScanActor_C|GetPostProcess (Variables|Default|GetScan%20Actor))
            (:Is%20Valid
              (Utilities|Struct|SetmembersinPostProcessSettings (Variables|/Script/Engine.PostProcessComponent|GetSettings (Variables|/Game/FX/BP_ScanActor.BP_ScanActor_C|GetPostProcess (Variables|Default|GetScan%20Actor))) (Utilities|Struct|MakeWeightedBlendables (Utilities|Array|MakeArray (Utilities|Struct|MakeWeightedBlendable 1.0 (Variables|Default|GetPPMID))))))))
        (:then_1
          (return (Variables|Default|GetScan%20Actor)))))))

(fn DestroyPPActor
  (if (and (Utilities|IsValid (Variables|Default|GetScan%20Actor)) (Variables|Default|GetbDestroyActor))
    (Actor|DestroyActor (Variables|Default|GetScan%20Actor))
    (Variables|Default|SetScan%20Actor 0)))

(fn UpdateScanPPBlendWeight
  (bind _blendcrv (Variables|Default|GetBlendCrv))
  (bind _scannormalizedtime (Variables|Default|GetScanNormalizedTime))
  (Utilities|IsValid _blendcrv
    (:Is%20Valid
      (LocalVariables|SetThisTime (Math|Curves|GetFloatValue _blendcrv _scannormalizedtime)))
    (:Is%20Not%20Valid
      (LocalVariables|SetThisTime _scannormalizedtime)))
  (bind _scanactor (CallFunction|GetScanPPActor))
  (Utilities|IsValid _scanactor
    (:Is%20Valid
      (Utilities|IsValid (Variables|/Game/FX/BP_ScanActor.BP_ScanActor_C|GetPostProcess _scanactor)
        (:Is%20Valid
          (Variables|/Script/Engine.PostProcessComponent|SetBlendWeight (Variables|/Game/FX/BP_ScanActor.BP_ScanActor_C|GetPostProcess _scanactor) (LocalVariables|GetThisTime)))))))

(fn UpdateScanLocation
  (bind _as_player_controller (Variables|Default|GetAs%20Player%20Controller))
  (bind _scan_actor (Variables|Default|GetScan%20Actor))
  (bind _returnvalue (Pawn|GetControlledPawn _as_player_controller))
  (bind _niagara (Variables|/Game/FX/BP_ScanActor.BP_ScanActor_C|GetNiagara _scan_actor))
  (bind _returnvalue_2 (Transformation|GetActorLocation _returnvalue))
  (Utilities|IsValid _as_player_controller
    (:Is%20Valid
      (Utilities|IsValid _returnvalue
        (:Is%20Valid
          (LocalVariables|SetThisLocation _returnvalue_2)
          (Rendering|Material|SetVectorParameterValue "/Game/FX/MPC_Scan.MPC_Scan" "Location" (Math|Conversions|ToLinearColor(Vector) _returnvalue_2) :!class /Script/Engine.KismetMaterialLibrary)
          (Utilities|IsValid _scan_actor
            (:Is%20Valid
              (Utilities|IsValid _niagara
                (:Is%20Valid
                  (Transformation|SetWorldLocation _niagara (Class|KismetMathLibrary|VectorSnappedtoGrid (LocalVariables|GetThisLocation) (Variables|Default|GetGridCellSize)) false false))))))))))